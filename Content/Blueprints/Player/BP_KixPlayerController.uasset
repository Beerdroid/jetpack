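; Player controller that handles Enhanced Input look, move, jump and jetpack flight for the possessed character, and creates its fuel overlay.
; Holding jetpack switches movement to Flying and adds upward thrust while fuel lasts; release or empty fuel restores Walking.
; Fuel checks, draining and jetpack start/stop go through messages to the character.
; Fuel values feed a BP_FuelVM view model shared with WBP_Overlay.
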(event `self.ReceiveBeginPlay`
  (`EnhancedInputSubsystemInterface.AddMappingContext` (subsystem `EnhancedInputLocalPlayerSubsystem`) "/Game/Blueprints/Input/IMC_KixMovement.IMC_KixMovement" 0 (struct))
  (`self.StoreEssentialVariables`)
  (`self.CreateOverlayWidget`))

(event `EnhancedInput|/Game/Blueprints/Input/InputActions/IA_Look`
  (params (ActionValue :type "Vector2D Structure") (ElapsedSeconds :type "Float (double-precision)") (TriggeredSeconds :type "Float (double-precision)") (InputAction :type "InputAction Object Reference" :default "/Game/Blueprints/Input/InputActions/IA_Look.IA_Look"))
  (:`Triggered`
    (`self.HandleLook`)))

(event `EnhancedInput|/Game/Blueprints/Input/InputActions/IA_Move`
  (params (ActionValue :type "Vector2D Structure") (ElapsedSeconds :type "Float (double-precision)") (TriggeredSeconds :type "Float (double-precision)") (InputAction :type "InputAction Object Reference" :default "/Game/Blueprints/Input/InputActions/IA_Move.IA_Move"))
  (:`Triggered`
    (`self.HandleMove`)))

(event `EnhancedInput|/Game/Blueprints/Input/InputActions/IA_Jump`
  (params (ActionValue :type Boolean) (ElapsedSeconds :type "Float (double-precision)") (TriggeredSeconds :type "Float (double-precision)") (InputAction :type "InputAction Object Reference" :default "/Game/Blueprints/Input/InputActions/IA_Jump.IA_Jump"))
  (:`Triggered`
    (`self.HandleJump`)))

(event `EnhancedInput|/Game/Blueprints/Input/InputActions/IA_JetPack`
  (params (ActionValue :type Boolean) (ElapsedSeconds :type "Float (double-precision)") (TriggeredSeconds :type "Float (double-precision)") (InputAction :type "InputAction Object Reference" :default "/Game/Blueprints/Input/InputActions/IA_JetPack.IA_JetPack"))
  (:`Triggered`
    (bind _controlledcharacter (`self.ControlledCharacter`)
      (:`then`
        (bind _hasfuel (message `/Game/Blueprints/Interfaces/BPI_Jetpack.HasFuel` _controlledcharacter))
        (if _hasfuel
          (`self.ApplyThrustInput`)
          (bind _residue (message `/Game/Blueprints/Interfaces/BPI_Jetpack.DrainJetFuel` (`self.ControlledCharacter`)))
          (`/Game/Blueprints/UI/BP_FuelVM.SetCurrentFuel` (`self.FuelViewModel`) _residue)
          (else
            (`/Engine/EditorBlueprintResources/StandardMacros.DoOnce` false :!label _label
              (:`Completed`
                (message `/Game/Blueprints/Interfaces/BPI_Jetpack.StopJetpack` (`self.ControlledCharacter`))
                (`self.StartWalking`))))))
      (:`else`)))
  (:`Started`
    (`self.StartJetPack`)
    (`self.ResetJetpackDoOnce`))
  (:`Completed`
    (if (`self.JetpackActive`)
      (`self.StopJetpack`))))

(event `ResetJetpackDoOnce`
  (goto _label :!via `Reset`))

(fn `ApplyThrustInput`
  (bind _controlledcharacter (`self.ControlledCharacter`)
    (:`then`
      (bind _movementcomponent (`self.MovementComponent`)
        (:`then`
          (`PawnMovementComponent.AddInputVector` _movementcomponent (* (`self.GetActorUpVector` _controlledcharacter) (`self.ThrusterFactorInput`)) false))
        (:`else`)))
    (:`else`)))

(fn `CreateOverlayWidget`
  (bind _returnvalue (`|GenericCreateObject` "/Game/Blueprints/UI/BP_FuelVM.BP_FuelVM_C"))
  (set `self.FuelViewModel` _returnvalue)
  (bind _returnvalue_2 (`|CreateWidget` "/Game/Blueprints/UI/WBP_Overlay.WBP_Overlay_C" self))
  (set `/Game/Blueprints/UI/WBP_Overlay.BP_FuelVM` (`self.FuelViewModel`) _returnvalue_2)
  (bind _output_get (set `self.OverlayWidget` _returnvalue_2))
  (`UserWidget.AddToViewport` _output_get 0))

(fn `HandleJump`
  (`self.ControlledCharacter`
    (:`then`
      (bind _ascharacter (cast `Character` (`self.K2_GetPawn`)))
      (`Character.Jump` _ascharacter))
    (:`else`)))

(fn `HandleLook`
  (bind (_x _y) (`KismetMathLibrary.BreakVector2D` (`|GetInputActionValue`)))
  (`self.AddYawInput` _x)
  (`self.AddPitchInput` _y))

(fn `HandleMove`
  (bind _returnvalue_x (`KismetMathLibrary.BreakVector2D` (`|GetInputActionValue`)))
  (bind (_returnvalue_x_2 _returnvalue_y) (`KismetMathLibrary.BreakVector2D` (`|GetInputActionValue`)))
  (`self.MovementComponent`
    (:`then`
      (`PawnMovementComponent.AddInputVector` (`self.MovementComponent`) (* _returnvalue_y (`KismetMathLibrary.GetForwardVector` (`self.GetControlRotation`))) false)
      (`PawnMovementComponent.AddInputVector` (`self.MovementComponent`) (* _returnvalue_x (`KismetMathLibrary.GetRightVector` (`self.GetControlRotation`))) false))
    (:`else`)))

(fn `StartFlying`
  (bind _movementcomponent (`self.MovementComponent`)
    (:`then`
      (`CharacterMovementComponent.SetMovementMode` _movementcomponent "MOVE_Flying" 0)
      (set `CharacterMovementComponent.bOrientRotationToMovement` false (`self.MovementComponent`))
      (set `CharacterMovementComponent.bUseControllerDesiredRotation` true (`self.MovementComponent`)))
    (:`else`)))

(fn `StartJetPack`
  (set `self.JetpackActive` true)
  (bind _controlledcharacter (`self.ControlledCharacter`)
    (:`then`
      (bind _hasfuel (message `/Game/Blueprints/Interfaces/BPI_Jetpack.HasFuel` _controlledcharacter))
      (if _hasfuel
        (message `/Game/Blueprints/Interfaces/BPI_Jetpack.StartJetpack` (`self.ControlledCharacter`))
        (`self.StartFlying`)))
    (:`else`)))

(fn `StartWalking`
  (bind _movementcomponent (`self.MovementComponent`)
    (:`then`
      (`CharacterMovementComponent.SetMovementMode` _movementcomponent "MOVE_Walking" 0)
      (set `CharacterMovementComponent.bOrientRotationToMovement` true (`self.MovementComponent`))
      (set `CharacterMovementComponent.bUseControllerDesiredRotation` false (`self.MovementComponent`)))
    (:`else`)))

(fn `StopJetpack`
  (set `self.JetpackActive` false)
  (bind _controlledcharacter (`self.ControlledCharacter`)
    (:`then`
      (message `/Game/Blueprints/Interfaces/BPI_Jetpack.StopJetpack` _controlledcharacter)
      (`self.StartWalking`))
    (:`else`)))

(fn `StoreEssentialVariables`
  (bind _ascharacter_movement_component (cast `CharacterMovementComponent` (`Pawn.GetMovementComponent` (`self.K2_GetPawn`))))
  (set `self.MovementComponent` _ascharacter_movement_component)
  (bind _ascharacter (cast `Character` (`self.K2_GetPawn`)))
  (set `self.ControlledCharacter` _ascharacter))

(fn `UpdateFuel`
  (params (FuelPercent :type "Float (double-precision)"))
  (`parent.UpdateFuel` FuelPercent)
  (`/Game/Blueprints/UI/BP_FuelVM.SetCurrentFuel` (`self.FuelViewModel`) (`local.FuelPercent`)))

(fn `UserConstructionScript`)