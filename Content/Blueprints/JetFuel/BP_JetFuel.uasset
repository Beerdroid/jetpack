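; BP_JetFuel is a fuel pickup that refills whatever actor overlaps it, then destroys itself.
; The overlap sends a RefillFuelMessage with its Fuel value to that actor, without filtering by type.
; Pickup effect and sound are soft references, played at its location if the effect is already loaded.
; Otherwise LoadPickUpEffect async-loads both and plays each on completion, though the actor is destroyed right after the request.
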(event `LoadPickUpEffect`
  (bind _pickupeffect (`self.PickUpEffect`))
  (bind _pickupsound (`self.PickUpSound`))
  (`|LoadAsset` _pickupeffect
    (:`then`
      (`|LoadAsset` _pickupsound
        (:`Completed`
          (`GameplayStatics.PlaySoundAtLocation` (`|ConvertAsset` _pickupsound) (`self.K2_GetActorLocation`) (struct) 0.5 1.0 0.0 null null null null))))
    (:`Completed`
      (`NiagaraFunctionLibrary.SpawnSystemAtLocation` (`|ConvertAsset` _pickupeffect) (`self.K2_GetActorLocation`)))))

(event `self.ReceiveActorBeginOverlap`
  (params (OtherActor :type "Actor Object Reference"))
  (message `/Game/Blueprints/Interfaces/BPI_Jetpack.RefillFuel` OtherActor (`self.Fuel`))
  (`/Engine/EditorBlueprintResources/StandardMacros.IsValid` (`|ConvertAsset` (`self.PickUpEffect`))
    (:`Is Valid`
      (`NiagaraFunctionLibrary.SpawnSystemAtLocation` (`|ConvertAsset` (`self.PickUpEffect`)) (`self.K2_GetActorLocation`))
      (`GameplayStatics.PlaySoundAtLocation` (`|ConvertAsset` (`self.PickUpSound`)) (`self.K2_GetActorLocation`) (struct) 0.5 1.0 0.0 null null null null))
    (:`Is Not Valid`
      (`self.LoadPickUpEffect`)))
  (`self.K2_DestroyActor`))

(fn `UserConstructionScript`)