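; Moving platform actor that travels back and forth continuously from BeginPlay.
; The PinPong timeline feeds its float track into InterpPlatformLocation, which is not defined in this graph, to update the platform's position.
; On finish, the timeline's direction selects PingPongForward or PingPongReverse, alternating PlayFromStart and ReverseFromEnd to form an endless loop without using Tick.
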(event `PingPongForward`
  (bind (_direction _float) (`Timeline|PinPong` :!via `PlayFromStart` :!label _label)
    (:`Update`
      (`self.InterpPlatformLocation` _float))
    (:`Finished`
      (switch `ETimelineDirection` _direction
        (:`Forward`
          (`self.PingPongReverse`))
        (:`Backward`
          (`self.PingPongForward`))))))

(event `PingPongReverse`
  (goto _label :!via `ReverseFromEnd`))

(event `self.ReceiveBeginPlay`
  (`parent.ReceiveBeginPlay`)
  (`self.PingPongForward`))

(fn `UserConstructionScript`
  (`parent.UserConstructionScript`))